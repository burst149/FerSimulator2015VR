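; Brightness controller that drives post-process auto-exposure bias from a timeline, apparently a time-of-day cycle.
; The Time timeline's Light track blends the bias, offset by Brightness, which the multiply and divide keys step up or down.
; Tick lowers Brightness from its high starting value while FadeIn is set, creating a fade from overexposure.
; Holding Add raises the near-frozen play rate with hold duration, and release drops it back.
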(event EventBeginPlay
  (Variables|Default|SetBrightness 1e+01)
  (Components|Timeline|SetPlayRate 0.001)
  (Components|Timeline|SetNewTime 17.0)
  (bind _light (Timeline|time Play)
    (:Update
      (Variables|/Script/Engine.PostProcessComponent|SetSettings (Variables|Default|GetPostProcess) (Utilities|Struct|MakePostProcessSettings true true true true true 0.03 2.0 1.0 8.0 (+ (Math|Float|Lerp -5.0 0.0 _light) (Variables|Default|GetBrightness)))))))

(event EventActorBeginOverlap
  (params (OtherActor :type Actor%20Object%20Reference)))

(event EventTick
  (params (DeltaSeconds :type Float%20%28single-precision%29))
  (bind _returnvalue (Game|GetPlayerController 0))
  (bind _returnvalue_2 (Class|PlayerController|GetInputKeyTimeDown _returnvalue "Add"))
  (if (> _returnvalue_2 0.0)
    (Components|Timeline|SetPlayRate (Math|Float|Clamp(Float) _returnvalue_2 0.0 2.0))
    (elif (< 0.001 (Components|Animation|GetPlayRate))
      (Components|Timeline|SetPlayRate (Math|Float|Clamp(Float) (- 0.0 (* DeltaSeconds 1e+01)) 0.001 5.0))))
  (if (Variables|Default|GetFadeIn)
    (bind _output_get (Variables|Default|SetBrightness (Math|Float|Clamp(Float) (- (Variables|Default|GetBrightness) (* 5.0 DeltaSeconds)) 0.0 1e+01)))
    (Variables|Default|SetFadeIn (> _output_get 0.0))))

(event Input|KeyboardEvents|Multiply
  (:Pressed
    (Variables|Default|SetBrightness (+ 0.5 (Variables|Default|GetBrightness)))))

(event Input|KeyboardEvents|Divide
  (:Pressed
    (Variables|Default|SetBrightness (+ (Variables|Default|GetBrightness) -0.5))))

(fn ConstructionScript)