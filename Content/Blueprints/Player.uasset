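; Player pawn for an Oculus VR game with movement, look, jump, trace-based interaction, orientation reset and aimed teleporting.
; Tick traces along the control rotation for a walkable spot, storing the destination and showing a marker while Teleport is held.
; Releasing Teleport on a valid spot ramps the camera's post-process exposure bias down as a fade-out, then moves the player.
; Escape quits the game.
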(event EventActorBeginOverlap
  (params (OtherActor :type Actor%20Object%20Reference)))

(event EventTick
  (params (DeltaSeconds :type Float%20%28single-precision%29))
  (bind _returnvalue (Transformation|GetActorLocation))
  (bind _returnvalue_2 (+ _returnvalue "0, 0,80.000000"))
  (Variables|/Script/Engine.CameraComponent|SetPostProcessSettings (Variables|Default|GetCamera) (Utilities|Struct|MakePostProcessSettings (Variables|Default|GetFadeOut) (Variables|Default|GetFade)))
  (Rendering|SetVisibility (Variables|Default|GetMarker) (and (Variables|Default|GetAimingTeleport) (Variables|Default|GetValidTeleport)) false)
  (if (Variables|Default|GetFadeOut)
    (if (> (Variables|Default|GetFade) -1e+01)
      (Variables|Default|SetFade (+ (Variables|Default|GetFade) (* -25.0 DeltaSeconds)))
      (else
        (Transformation|Teleport (Variables|Default|GetTeleportOffest) "0.000000, 0,0.000000")
        (Variables|Default|SetFadeOut false)))
    (else
      (if (< (Variables|Default|GetFade) 0.0)
        (Variables|Default|SetFade (+ (Variables|Default|GetFade) (* 25.0 DeltaSeconds))))
      (bind _outhit (Collision|LineTraceByChannel _returnvalue_2 (+ _returnvalue_2 (* (Math|Vector|GetForwardVector (Pawn|GetControlRotation :!class /Script/Engine.Pawn)) 5e+03)) "TraceTypeQuery1" false 0 "None"))
      (if (Class|CharacterMovementComponent|IsWalkable _outhit)
        (Transformation|SetWorldLocation (Variables|Default|GetMarker) (+ "0, 0,-88.000000" (+ (.Location (Collision|BreakHitResult _outhit)) "0, 0,88.000000")) false)
        (Variables|Default|SetTeleportOffest (+ (.Location (Collision|BreakHitResult _outhit)) "0, 0,88.000000"))
        (Variables|Default|SetValidTeleport true)
        (else
          (Variables|Default|SetValidTeleport false))))))

(event EventBeginPlay
  (Variables|Default|SetFade -4e+01)
  (Class|HeadMountedDisplayFunctionLibrary|EnableLowPersistenceMode true))

(event Input|ActionEvents|InputActionJump
  (:Pressed
    (Character|Jump)))

(event Input|ActionEvents|InputActionTeleport
  (:Pressed
    (Variables|Default|SetAimingTeleport true))
  (:Released
    (Variables|Default|SetAimingTeleport false)
    (if (Variables|Default|GetValidTeleport)
      (Variables|Default|SetFadeOut true))))

(event Input|ActionEvents|InputActionResetOculus
  (:Released
    (Class|HeadMountedDisplayFunctionLibrary|ResetOrientationandPosition 0.0 "OrientationAndPosition")))

(event Input|ActionEvents|InputActionInteract
  (bind _returnvalue (Transformation|GetActorLocation))
  (bind _returnvalue_2 (+ _returnvalue "0, 0,100.000000"))
  (:Pressed
    (bind (_outhit _returnvalue_3) (Collision|LineTraceByChannel _returnvalue_2 (+ _returnvalue_2 (* (Math|Vector|GetForwardVector (Pawn|GetControlRotation :!class /Script/Engine.Pawn)) 2.5e+02)) "TraceTypeQuery1" false 0 "None"))
    (if _returnvalue_3
      (Class|Interactable|Interact(Message) (.HitActor (Collision|BreakHitResult _outhit))))))

(event Input|AxisEvents|InputAxisCameraForward
  (params (AxisValue :type Float%20%28single-precision%29))
  (Pawn|Input|AddMovementInput (Math|Vector|GetForwardVector (Transformation|GetActorRotation)) AxisValue false))

(event Input|AxisEvents|InputAxisCameraRight
  (params (AxisValue :type Float%20%28single-precision%29))
  (Pawn|Input|AddMovementInput (Math|Vector|GetRightVector (Transformation|GetActorRotation)) AxisValue false))

(event Input|AxisEvents|InputAxisCameraPitch
  (params (AxisValue :type Float%20%28single-precision%29))
  (Pawn|Input|AddControllerPitchInput AxisValue))

(event Input|AxisEvents|InputAxisCameraYaw
  (params (AxisValue :type Float%20%28single-precision%29))
  (Pawn|Input|AddControllerYawInput AxisValue))

(event Input|KeyboardEvents|Escape
  (:Pressed
    (Game|QuitGame 0 "Quit")))

(fn ConstructionScript)